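; Spear actor for the phase 1 light ranged attack, which dissolves in with a fire effect when spawned.
; SpawnDissolve timeline drives the dissolve amount and color, calling CheckForSpears on each update to count SpearChecker-class actors.
; When the last array index exceeds 1, this spear restarts EndDissolve, which fades it out, then stops the fire and destroys it.
; NewMacro_0 is an unfinished spear-lookup macro that the graph never uses.
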(event `self.ReceiveBeginPlay`
  (bind _spear (`self.Spear`))
  (`PrimitiveComponent.SetMaterial` _spear 0 "/Game/Effects/Planar_Dissolve/MAT_Dissolver_Test.MAT_Dissolver_Test")
  ;[0.1962 0.2344 0.07682] Activate Spear
  (`ActorComponent.Activate` (`self.Spear_Fire`) false)
  (bind (_direction _appear_spear _appear_color) (`Timeline|Spawn Dissolve`)
    (:`Update`
      (`MeshComponent.SetScalarParameterValueOnMaterials` _spear "D_Amount" _appear_spear)
      (`MeshComponent.SetVectorParameterValueOnMaterials` _spear "Color" (`KismetMathLibrary.Conv_LinearColorToVector` _appear_color))
      (bind _killtrue (`self.CheckForSpears`))
      (if _killtrue
        ;[1 1 1] Fade Out
        (bind (_direction_2 _kill_dissolver) (`Timeline|End Dissolve` :!via `PlayFromStart`)
          (:`Update`
            (`MeshComponent.SetScalarParameterValueOnMaterials` (`self.Spear`) "D_Amount" _kill_dissolver))
          (:`Finished`
            (`ActorComponent.Deactivate` (`self.Spear_Fire`))
            (`self.K2_DestroyActor`)))))))

(event `self.ProjectileMovement.OnProjectileStop`
  (params (ImpactResult :type "HitResult Structure (by ref)")))

(fn `CheckForSpears`
  (returns (KillTrue :type Boolean))
  (locals (`Spear Checker` :type "Actor Class Reference" :default "BlueprintGeneratedClass'/Game/Effects/Light_Ranged_Attack/bp_Light_RA_ph1.bp_Light_RA_ph1_C'") (AllSpears :type "Array of Actor Object Reference"))
  (bind _outactors (`GameplayStatics.GetAllActorsOfClass` (`local.Spear Checker`)))
  (bind _output_get (set `local.AllSpears` _outactors))
  (for (_ _array_index) _output_get
    _)
  (if (> _array_index 1)
    (return true)
    (else
      (return false))))

(fn `UserConstructionScript`
  (locals (`This Spear` :type "Actor Class Reference")))