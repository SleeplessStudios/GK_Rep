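; A skydome cloud Blueprint from the effects kit that groups twelve cloud components.
; Its construction script assigns the MIN_Clouds_03_Ray material to slot 0 of all twelve clouds.
; It has no runtime logic, as the event graph holds only disabled default events.
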(fn `UserConstructionScript`
  (`PrimitiveComponent.SetMaterial` (`|MakeArray` (`self.Cloud_01`) (`self.Cloud_02`) (`self.Cloud_03`) (`self.Cloud_04`) (`self.Cloud_05`) (`self.Cloud_06`) (`self.Cloud_07`) (`self.Cloud_08`) (`self.Cloud_09`) (`self.Cloud_10`) (`self.Cloud_11`) (`self.Cloud_12`) :!type "PrimitiveComponent Object Reference") 0 "/Game/Effects/kit_Skydome/MIN_Clouds_03_Ray.MIN_Clouds_03_Ray"))