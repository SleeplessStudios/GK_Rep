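; Sky dome actor that layers an HDR sky, scrolling back and front cloud textures, and rotating cloud meshes.
; The construction script creates dynamic material instances for the dome and front cloud mesh, pushing exposed size, offset, HDR, tiling, speed, opacity and color settings into them.
; BeginPlay spawns a Bp_Clouds_02 actor, attaches it to CloudsDirectionArrow and scales it.
; Tick yaws OriginCloudsCube at MeshCloudsRotationSpeed, scaled by delta time.
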(event `self.ReceiveBeginPlay`
  ;[0.2998 0.4988 1] Spawn 1 BP
  (bind _returnvalue (`|SpawnActorFromClass` "/Game/Effects/kit_Skydome/Clouds/bp_Clouds_02.bp_Clouds_02_C" (`KismetMathLibrary.Conv_VectorToTransform` (+ (`SceneComponent.K2_GetComponentLocation` (`self.Clouds_Direction_Arrow`)) (`self.Mesh Cloud Offset`))) "Undefined" "OverrideRootScale" null null))
  (bind _rootcomponent (`Actor.RootComponent` _returnvalue))
  (`SceneComponent.K2_AttachToComponent` _rootcomponent (`self.Clouds_Direction_Arrow`) "None" "KeepRelative" "KeepRelative" "KeepRelative" true)
  (`SceneComponent.SetWorldScale3D` _rootcomponent (`self.Mesh Cloud Scale`)))

(event `self.ReceiveTick`
  (params (DeltaSeconds :type "Float (single-precision)"))
  ;[0 0.8673 1] Clouds Rotation OverTime
  (`SceneComponent.K2_AddLocalRotation` (`self.Origin_Clouds_Cube`) (* (`KismetMathLibrary.MakeRotator` 0.0 0.0 (`self.Mesh Clouds Rotation Speed`)) DeltaSeconds) false false))

(fn `UserConstructionScript`
  (`|ExecutionSequence`
    (:`then_0`
      (bind _returnvalue (`PrimitiveComponent.CreateDynamicMaterialInstance` (`self.sm_SkyDome_Mesh`) 0 "/Game/Effects/kit_Skydome/Resources/MAST_Sky_Dome.MAST_Sky_Dome"))
      ;[0.2289 0 1] Sky Dome
      (`SceneComponent.SetWorldScale3D` (`self.sm_SkyDome_Mesh`) (`self.SkyDome Size`))
      (`MaterialInstanceDynamic.SetScalarParameterValue` _returnvalue "HDR Power" (`self.HDR Power`))
      (`MaterialInstanceDynamic.SetScalarParameterValue` _returnvalue "HDR Intensity" (`self.HDR Intensity`))
      ;[0 0.437 1] Back Clouds Texture
      (`MaterialInstanceDynamic.SetScalarParameterValue` _returnvalue "Back Clouds X Speed" (`self.BackClouds X Speed`))
      (`MaterialInstanceDynamic.SetScalarParameterValue` _returnvalue "Back Clouds Y Speed" (`self.BackClouds Y Speed`))
      (`MaterialInstanceDynamic.SetScalarParameterValue` _returnvalue "Back Clouds U Tile" (`self.BackClouds U Tile`))
      (`MaterialInstanceDynamic.SetScalarParameterValue` _returnvalue "Back Clouds V Tile" (`self.BackClouds V Tile`))
      (`MaterialInstanceDynamic.SetScalarParameterValue` _returnvalue "Back Clouds Opacity" (`self.BackClouds Opacity`))
      (`MaterialInstanceDynamic.SetScalarParameterValue` _returnvalue "Back Clouds V Offset" (`self.BackClouds V Offset`))
      (`MaterialInstanceDynamic.SetScalarParameterValue` _returnvalue "Back Clouds U Offset" (`self.BackClouds U Offset`))
      (`MaterialInstanceDynamic.SetVectorParameterValue` _returnvalue "Back Clouds Color" (`self.Back Clouds Color`)))
    (:`then_1`
      (bind _returnvalue_2 (`PrimitiveComponent.CreateDynamicMaterialInstance` (`self.sm_Sky_Front_Clouds`) 0 "/Game/Effects/kit_Skydome/Resources/MAST_Front_Clouds.MAST_Front_Clouds"))
      ;[0.2773 0.3748 1] Front Cloud Mesh
      (`SceneComponent.K2_SetRelativeLocation` (`self.sm_Sky_Front_Clouds`) (`self.Front Clouds Offset`) false false)
      ;[0.299 0.4433 1] Front Clouds Texture
      (`MaterialInstanceDynamic.SetScalarParameterValue` _returnvalue_2 "Front Clouds X Speed" (`self.FrontClouds X Speed`))
      (`MaterialInstanceDynamic.SetScalarParameterValue` _returnvalue_2 "Front Clouds Y Speed" (`self.FrontClouds Y Speed`))
      (`MaterialInstanceDynamic.SetScalarParameterValue` _returnvalue_2 "Front Clouds U Tile" (`self.FrontClouds U Tile`))
      (`MaterialInstanceDynamic.SetScalarParameterValue` _returnvalue_2 "Front Clouds V Tile" (`self.FrontClouds V Tile`))
      (`MaterialInstanceDynamic.SetScalarParameterValue` _returnvalue_2 "Front Clouds V Offset" (`self.FrontClouds V Offset`))
      (`MaterialInstanceDynamic.SetScalarParameterValue` _returnvalue_2 "Front Clouds U Offset" (`self.FrontClouds U Offset`))
      (`MaterialInstanceDynamic.SetScalarParameterValue` _returnvalue_2 "Front Clouds Opacity" (`self.FrontClouds Opacity`))
      (`MaterialInstanceDynamic.SetVectorParameterValue` _returnvalue_2 "Front Clouds Color" (`self.Front Clouds Color`)))))