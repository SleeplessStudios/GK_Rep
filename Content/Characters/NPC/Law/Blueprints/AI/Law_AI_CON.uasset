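; Law_AI_CON is the AI controller for the Law NPC, running Law_Tree on Law_Blackboard.
; BeginPlay seeds the blackboard with the player's location and the controlled BP_Law pawn's NextLocation, which is written only once.
; Tick keeps focus on the player and refreshes PlayerLocation every frame.
; Its final check of the pawn's InRange flag leads to no action.
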(event `self.ReceiveBeginPlay`
  (`self.UseBlackboard` "/Game/Characters/NPC/Law/Blueprints/AI/Law_Blackboard.Law_Blackboard")
  (`BlackboardComponent.SetValueAsVector` (`AIBlueprintHelperLibrary.GetBlackboard` self) (`self.PlayerLocation`) (`self.K2_GetActorLocation` (`GameplayStatics.GetPlayerCharacter` 0)))
  (`self.RunBehaviorTree` "/Game/Characters/NPC/Law/Blueprints/AI/Law_Tree.Law_Tree")
  (bind _asbp_law (cast `/Game/Characters/NPC/Law/Blueprints/BP_Law` (`self.K2_GetPawn`)))
  (`BlackboardComponent.SetValueAsVector` (`AIBlueprintHelperLibrary.GetBlackboard` null) (`self.NextLocation`) (`/Game/Characters/NPC/Law/Blueprints/BP_Law.NextLocation` _asbp_law)))

(event `self.ReceiveTick`
  (params (DeltaSeconds :type "Float (single-precision)"))
  (`self.K2_SetFocus` (`GameplayStatics.GetPlayerCharacter` 0))
  (`BlackboardComponent.SetValueAsVector` (`AIBlueprintHelperLibrary.GetBlackboard` self) (`self.PlayerLocation`) (`self.K2_GetActorLocation` (`GameplayStatics.GetPlayerCharacter` 0)))
  (bind _asbp_law (cast `/Game/Characters/NPC/Law/Blueprints/BP_Law` (`self.K2_GetPawn`)))
  (if (`/Game/Characters/NPC/Law/Blueprints/BP_Law.In Range` _asbp_law)
    _))

(fn `UserConstructionScript`)