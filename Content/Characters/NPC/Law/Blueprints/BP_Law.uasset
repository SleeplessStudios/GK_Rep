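; BP_Law is an enemy NPC character that hunts and attacks the player.
; Tick ramps up walk speed and picks by distance: attack when close, pursue via AI SimpleMoveTo at mid range, or teleport beside the player when far.
; Attacks play a three-step montage combo with buffering and speed reset; hammer and unarmed branches currently share montages.
; Hits briefly swap the material, then apply damage, destroying the actor at zero health.
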(event `Teleport`
  ;[0.9266 1 0] Teleport
  (if (`self.Teleporting`)
    (`AnimInstance.Montage_Play` (`SkeletalMeshComponent.GetAnimInstance` (`self.Mesh`)) null 1.0 "MontageLength" 0.0 true)))

(event `self.ReceiveTick`
  (params (DeltaSeconds :type "Float (single-precision)"))
  ;[0 1 0.113] If in Range - Attack Player
  (`self.IncreaseSpeed`)
  (set `CharacterMovementComponent.MaxWalkSpeed` (`self.Current Speed`) (`self.CharacterMovement`))
  (bind _distancefromplayer (`self.Distance From Player Check`))
  (if (< _distancefromplayer 1000.0)
    (set `self.In Range` true)
    ;[0.9266 1 0] Teleport
    (`self.AttackTarget`)
    (elif (> _distancefromplayer 2000.0)
      (`self.TeleportLaw`)
      (else
        (`self.MoveTowardsPlayer`)
        (set `self.In Range` false)))))

(event `Hit`
  (bind _mesh (`self.Mesh`))
  ;[1 0 0.7898] Hit Feedback
  (`PrimitiveComponent.SetMaterial` _mesh 0 "/Game/Characters/NPC/Law/Materials/Law_Weapon_Mat.Law_Weapon_Mat")
  (`KismetSystemLibrary.Delay` 0.5)
  (`PrimitiveComponent.SetMaterial` _mesh 0 "/Game/Characters/NPC/Law/Materials/lambert17.lambert17")
  (`self.TakeDamage` 5.0))

(event `SaveComboAttack`
  ;[0 0.008406 1] Attack System
  ;;[1 0 0] Save Combo
  (if (`self.Save Attack`)
    (set `self.Save Attack` false)
    (if (`self.Hammer Equipped`) :!label _label
      (`self.Hammer Combo`)
      (else
        (`self.No Hammer Combo`)))))

(event `AttackTarget`
  ;[0 0.008406 1] Attack System
  (if (`self.Is Attacking`)
    (set `self.Save Attack` true)
    (else
      (set `self.Is Attacking` true)
      (if (`self.Charging`)
        ;[1 0.03182 0] Charging
        (`AnimInstance.Montage_Play` (`SkeletalMeshComponent.GetAnimInstance` (`self.Mesh`)) null 1.0 "MontageLength" 0.0 true)
        (else
          (goto _label))))))

(event `Hammer Equip/Unequip`
  (`/Engine/EditorBlueprintResources/StandardMacros.FlipFlop`
    (:`A`
      (set `self.Hammer Equipped` true))
    (:`B`
      (set `self.Hammer Equipped` false))))

(event `ResetCombo`
  ;[0 0 0] Reset Combo
  (set `self.Save Attack` false)
  (set `self.ComboCounter` 0)
  (set `self.Is Attacking` false)
  (set `self.Charging` false)
  (set `self.Teleporting` false))

(fn `AttachWeapon`)

(fn `Distance From Player Check`
  (returns (DistanceFromPlayer :type "Float (double-precision)"))
  (return (`self.GetDistanceTo` (`GameplayStatics.GetPlayerCharacter` 0))))

(fn `GetHealth`
  (returns (ReturnValue :type "Float (double-precision)"))
  (return 0.0))

(fn `Hammer Combo`
  (bind _currentcombo (`self.CurrentCombo`))
  (switch `int` (`self.ComboCounter`)
    (:`0`
      (set `self.ComboCounter` 1)
      (set `self.CurrentCombo` "/Game/Characters/NPC/Law/Animations/Montages/Law_LightAttack_01_V3_AM.Law_LightAttack_01_V3_AM"))
    (:`1`
      (set `self.ComboCounter` 2)
      (set `self.CurrentCombo` "/Game/Characters/NPC/Law/Animations/Montages/Law_LightAttack_02_V2_AM.Law_LightAttack_02_V2_AM"))
    (:`2`
      (set `self.ComboCounter` 3)
      (set `self.CurrentCombo` "/Game/Characters/NPC/Law/Animations/Montages/Law_RunningHeavy_AM.Law_RunningHeavy_AM")))
  (`AnimInstance.Montage_Play` (`SkeletalMeshComponent.GetAnimInstance` (`self.Mesh`)) _currentcombo 1.0 "MontageLength" 0.0 true)
  (`KismetSystemLibrary.PrintString` (`KismetSystemLibrary.GetDisplayName` _currentcombo))
  (set `self.Current Speed` 0.0))

(fn `HealthManager`
  (bind _output_get (set `self.Health` (`self.Health`)))
  (if (<= _output_get 0.0)
    (`self.K2_DestroyActor`)))

(fn `IncreaseSpeed`
  (bind _current_speed (`self.Current Speed`))
  (`KismetSystemLibrary.PrintString` (`KismetStringLibrary.Conv_DoubleToString` _current_speed))
  (set `self.Current Speed` (`KismetMathLibrary.FInterpTo` _current_speed 375.0 (`GameplayStatics.GetWorldDeltaSeconds`) 0.25)))

(fn `No Hammer Combo`
  (bind _currentcombo (`self.CurrentCombo`))
  (switch `int` (`self.ComboCounter`)
    (:`0`
      (set `self.ComboCounter` 1)
      (set `self.CurrentCombo` "/Game/Characters/NPC/Law/Animations/Montages/Law_LightAttack_01_V3_AM.Law_LightAttack_01_V3_AM"))
    (:`1`
      (set `self.ComboCounter` 2)
      (set `self.CurrentCombo` "/Game/Characters/NPC/Law/Animations/Montages/Law_LightAttack_02_V2_AM.Law_LightAttack_02_V2_AM"))
    (:`2`
      (set `self.ComboCounter` 3)
      (set `self.CurrentCombo` "/Game/Characters/NPC/Law/Animations/Montages/Law_RunningHeavy_AM.Law_RunningHeavy_AM")))
  (`AnimInstance.Montage_Play` (`SkeletalMeshComponent.GetAnimInstance` (`self.Mesh`)) _currentcombo 1.0 "MontageLength" 0.0 true)
  (`KismetSystemLibrary.PrintString` (`KismetSystemLibrary.GetDisplayName` _currentcombo))
  (set `self.Current Speed` 0.0))

(fn `TakeDamage`
  (params (Damage :type "Float (double-precision)"))
  (set `self.Health` (- (`self.Health`) Damage))
  (`self.HealthManager`))

(fn `TeleportLaw`
  (`self.K2_TeleportTo` (- (`self.K2_GetActorLocation` (`GameplayStatics.GetPlayerCharacter` 0)) 75.0))
  (`AnimInstance.Montage_Play` (`SkeletalMeshComponent.GetAnimInstance` (`self.Mesh`)) "/Game/Characters/NPC/Law/Animations/Montages/Law_Teleport_Land_AM.Law_Teleport_Land_AM" 1.0 "MontageLength" 0.0 true))

(fn `UserConstructionScript`
  (`parent.UserConstructionScript`)
  (`self.AttachWeapon`))

(fn `Walking`
  (set `CharacterMovementComponent.MaxWalkSpeed` (* 0.0 0.0) (`self.CharacterMovement`)))