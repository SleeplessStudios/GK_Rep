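; AI controller for the Creep NPC that starts its behavior tree and keeps it focused on the player.
; On BeginPlay it sets up the Creep_Data blackboard, seeds PlayerLocation with the controlled pawn's own location, then runs Creep_BTree.
; Every Tick it sets focus to the first player character.
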(event `self.ReceiveBeginPlay`
  (`self.UseBlackboard` "/Game/Characters/NPC/Creep/Blueprints/AI/Creep_Data.Creep_Data")
  (`BlackboardComponent.SetValueAsVector` (`AIBlueprintHelperLibrary.GetBlackboard` self) (`self.PlayerLocation`) (`self.K2_GetActorLocation` (`self.K2_GetPawn`)))
  (`self.RunBehaviorTree` "/Game/Characters/NPC/Creep/Blueprints/AI/Creep_BTree.Creep_BTree"))

(event `self.ReceiveTick`
  (params (DeltaSeconds :type "Float (single-precision)"))
  (`self.K2_SetFocus` (`GameplayStatics.GetPlayerCharacter` 0)))

(fn `UserConstructionScript`)