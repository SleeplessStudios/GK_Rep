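; BP_Creep is a creep NPC that can be lock-on targeted and damaged.
; Each TargetLockON call toggles TargetVisual through a FlipFlop, and AffectHealth feeds HealthManager, which subtracts damage and sets IsDead at zero health or below.
; The Construction Script tints the mesh red through a dynamic material, and a helper returns distance to the player.
; The IsDead branch after damage is empty, so death has no further effect here.
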(event `/Game/Maps/Game_BPI.TargetLockON`
  (bind _target_visual (`self.Target Visual`))
  (`/Engine/EditorBlueprintResources/StandardMacros.FlipFlop`
    (:`A`
      (`SceneComponent.SetHiddenInGame` _target_visual false false))
    (:`B`
      (`SceneComponent.SetHiddenInGame` _target_visual true false))))

(event `/Game/Maps/iDamageable.Affect Health`
  (params (Damage :type "Float (single-precision)"))
  (`self.HealthManager` Damage)
  (if (`self.Is Dead`)
    _))

(fn `DistanceFromPlayer`
  (returns (Distance :type "Float (double-precision)"))
  (return (`self.GetDistanceTo` (`GameplayStatics.GetPlayerCharacter` 0))))

(fn `HealthManager`
  (params (Damage :type "Float (double-precision)"))
  (set `self.Current Health` (- (`self.Current Health`) Damage))
  (if (<= (`self.Current Health`) 0.0)
    (set `self.Is Dead` true)))

(fn `UserConstructionScript`
  (locals (`Dyn Mat` :type "MaterialInstanceDynamic Object Reference"))
  (bind _returnvalue (`PrimitiveComponent.CreateDynamicMaterialInstance` (`self.Mesh`) 0 null))
  (bind _output_get (set `local.Dyn Mat` _returnvalue))
  (`MaterialInstanceDynamic.SetVectorParameterValue` _output_get "BodyColor" (struct :`R` 1.0 :`B` 0.009549 :`A` 1.0)))