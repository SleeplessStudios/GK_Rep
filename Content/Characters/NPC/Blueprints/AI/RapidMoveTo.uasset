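; RapidMoveTo is a Behavior Tree task that moves a follower NPC toward the actor stored in its TargetToFollow blackboard key.
; On execute, it casts the owner to Follower_AI_CON and caches that controller, reusing the reference on later runs.
; It runs AI MoveTo on the controlled pawn with a tight acceptance radius.
; The task finishes only when the move succeeds; move failure and a failed cast never call FinishExecute.
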(event `self.ReceiveExecute`
  (params (OwnerActor :type "Actor Object Reference"))
  ;[1 1 1] Is AI_FOLLOWER_CON?
  (if (not (!= (`self.AI_CON_Ref`) null))
    (bind _asfollower_ai_con (cast `/Game/Characters/NPC/Blueprints/AI/Follower_AI_CON` OwnerActor))
    (set `self.AI_CON_Ref` _asfollower_ai_con))
  (`|AIMoveTo` (`Controller.K2_GetPawn` (`self.AI_CON_Ref`)) (0.0 0.0 0.0) (`BTFunctionLibrary.GetBlackboardValueAsActor` (`self.TargetToFollow`)) 10.0
    (:`OnSuccess`
      (`self.FinishExecute` true))))