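; BP_Law is an NPC melee fighter that plays an attack montage when the player comes within range.
; Tick checks player distance and drives a combo-buffer state, though the counter never advances and only the first step is handled.
; Hit briefly swaps the mesh material, then applies damage, and the actor is destroyed at zero health.
; Events toggle weapon collision, but the overlap and socket-attach logic are disconnected.
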(event `SaveComboAttack`
  (if (`self.SaveAttack`)
    (set `self.SaveAttack` false)
    (`KismetSystemLibrary.Delay` 2.5 :!label _label)
    (set `self.Is Attacking` false)))

(event `ResetCombo`
  (set `self.ComboCounter` 0)
  (set `self.SaveAttack` false)
  (set `self.Is Attacking` false))

(event `self.ReceiveTick`
  (params (DeltaSeconds :type "Float (single-precision)"))
  ;[1 1 1] Light Attack
  (bind _distancefromplayer (`self.Distance From Player Check`))
  (if (<= _distancefromplayer 1000.0)
    (if (`self.Is Attacking`)
      (set `self.SaveAttack` true)
      (goto _label)
      (else
        (set `self.Is Attacking` true)
        (switch `int` (`self.ComboCounter`)
          (:`0`
            (set `self.ComboCounter` (`self.ComboCounter`))
            (bind _output_get (set `self.CurrentCombo` (`self.CurrentCombo`)))
            (`AnimInstance.Montage_Play` (`SkeletalMeshComponent.GetAnimInstance` (`self.Mesh`)) _output_get 1.0 "MontageLength" 0.0 true)))))))

(event `self.ReceiveBeginPlay`
  (`self.HealthManager`)
  (`self.CollideOff`))

(event `CollideOff`
  ;[1 1 1] Collision Manager
  (`PrimitiveComponent.SetCollisionEnabled` (`self.Weapon`) "NoCollision"))

(event `CollideOn`
  ;[1 1 1] Collision Manager
  (`PrimitiveComponent.SetCollisionEnabled` (`self.Weapon`) "QueryAndPhysics"))

(event `Hit`
  (bind _mesh (`self.Mesh`))
  ;[1 1 1] Hit Feedback
  (`PrimitiveComponent.SetMaterial` _mesh 0 "/Game/Characters/NPC/Materials/Law_Weapon_Mat.Law_Weapon_Mat")
  (`KismetSystemLibrary.Delay` 0.5)
  (`PrimitiveComponent.SetMaterial` _mesh 0 "/Game/Characters/NPC/Materials/lambert17.lambert17")
  (`self.TakeDamage` 5.0))

(event `self.Weapon.OnComponentBeginOverlap`
  (params (OverlappedComponent :type "PrimitiveComponent Object Reference") (OtherActor :type "Actor Object Reference") (OtherComp :type "PrimitiveComponent Object Reference") (OtherBodyIndex :type Integer) (bFromSweep :type Boolean) (SweepResult :type "HitResult Structure (by ref)")))

(fn `AttachWeapon`)

(fn `Distance From Player Check`
  (returns (DistanceFromPlayer :type "Float (double-precision)"))
  (return (`self.GetDistanceTo` (`GameplayStatics.GetPlayerCharacter` 0))))

(fn `GetHealth`
  (returns (ReturnValue :type "Float (double-precision)"))
  (return 0.0))

(fn `HealthManager`
  (bind _output_get (set `self.Health` (`self.Health`)))
  (if (<= _output_get 0.0)
    (`self.K2_DestroyActor`)))

(fn `TakeDamage`
  (params (Damage :type "Float (double-precision)"))
  (set `self.Health` (- (`self.Health`) Damage))
  (`self.HealthManager`))

(fn `UserConstructionScript`
  (`parent.UserConstructionScript`)
  (`self.AttachWeapon`))

(fn `Walking`
  (set `CharacterMovementComponent.MaxWalkSpeed` (* (`self.speedRate`) (`self.speedVariable`)) (`self.CharacterMovement`)))